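; Base weapon actor that acts as a proximity-based pickup prompt for the player.
; When MyCharacter begins overlapping the Collider, it tells that character to show an equip message, passing the weapon's Name and a self reference.
; Ending the overlap hides the message.
; The logic that would add the weapon to the character's Weapons array is disconnected and never runs.
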(event OnComponentBeginOverlap(Collider)
  (params (OverlappedComponent :type Primitive%20Component%20Object%20Reference) (OtherActor :type Actor%20Object%20Reference) (OtherComp :type Primitive%20Component%20Object%20Reference) (OtherBodyIndex :type Integer) (bFromSweep :type Boolean) (SweepResult :type Hit%20Result%20Structure%20%28by%20ref%29))
  ;[1 1 1] Text is shown when touching
  (bind _asmy_character (Utilities|Casting|CastToMyCharacter OtherActor))
  (Class|HUDInterface|ShowEquipMessage(Message) _asmy_character (Variables|Default|Getname) self))

(event OnComponentEndOverlap(Collider)
  (params (OverlappedComponent :type Primitive%20Component%20Object%20Reference) (OtherActor :type Actor%20Object%20Reference) (OtherComp :type Primitive%20Component%20Object%20Reference) (OtherBodyIndex :type Integer))
  ;[1 1 1] If not touching weapon
  (bind _asmy_character (Utilities|Casting|CastToMyCharacter OtherActor))
  (Class|HUDInterface|HideEquipMessage(Message) _asmy_character))

(event EventBeginPlay)

(event EventTick
  (params (DeltaSeconds :type Float%20%28single-precision%29)))

(event Collision|EventActorBeginOverlap
  (params (OtherActor :type Actor%20Object%20Reference))
  ;[1 1 1] If touching adds to array
)

(fn ConstructionScript)